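; BP_FINALD is a final door that opens once all BP_CollectableItem actors in the level have been collected.
; BeginPlay counts those items, and each ItemCollected call decrements the count, triggering OpenDoor at zero or immediately if none exist.
; A Timeline lerps the Arrow component's yaw from closed to open.
; Its Update also plays a 2D sound and runs a five-second Delay before destroying the actor.
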(event `OpenDoor`
  (bind (_direction _newtrack_puerta) (`Timeline|Timeline`)
    (:`Update`
      (`SceneComponent.K2_SetRelativeRotation` (`self.Arrow`) (`KismetMathLibrary.MakeRotator` 0.0 0.0 (`KismetMathLibrary.Lerp` (`self.Puerta Cerrada`) (`self.Puerta Abierta`) _newtrack_puerta)) false false)
      (`GameplayStatics.PlaySound2D` "/Game/GamePlay_Elements/Puerta/opendoor.opendoor" 1.0 1.0 0.0 null null)
      (`KismetSystemLibrary.Delay` 5.0)
      (`self.K2_DestroyActor`))))

(event `self.ReceiveBeginPlay`
  (bind _outactors (`GameplayStatics.GetAllActorsOfClass` "/Game/GamePlay_Elements/Coleccionables/BP_CollectableItem.BP_CollectableItem_C"))
  (bind _output_get (set `self.RemainingCollectableItem` (`KismetArrayLibrary.Array_Length` _outactors)))
  (if (== _output_get 0)
    (`self.OpenDoor`)))

(event `ItemCollected`
  (bind _result (`/Engine/EditorBlueprintResources/StandardMacros.DecrementInt` (`self.RemainingCollectableItem`))
    (:`  `
      (if (== _result 0)
        (`self.OpenDoor`)))))

(fn `UserConstructionScript`)